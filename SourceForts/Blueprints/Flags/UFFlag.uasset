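; Team-colored capture-the-flag actor that can sit at its home stand, ride above a carrier or lie dropped as a physics object.
; OnRep of FlagState switches attachment and physics, while the authority runs a reset timer for drops that sets Home's state to Base.
; Touching a dropped flag, after a brief grace period, returns it for teammates or gives it to opponents through UFFlagStand.
; If destroyed, it has Home create a replacement.
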(event OnComponentBeginOverlap(Sphere)
  (params (OtherActor :type Actor%20Object%20Reference) (OtherComp :type Primitive%20Component%20Object%20Reference) (OtherBodyIndex :type Integer) (bFromSweep :type Boolean) (SweepResult :type Hit%20Result%20Structure%20%28by%20ref%29))
  (Utilities|CheckFlagState
    (:Dropped
      (if (not (Variables|UFRestricted|GetbRecentDrop))
        (bind _asufcharacter (Utilities|Casting|CastToUFCharacter OtherActor))
        (if (== (Class|UTCharacter|GetTeamNum _asufcharacter) (Variables|UFRestricted|GetTeamNum))
          (bind _asufflag_stand (Utilities|Casting|CastToUFFlagStand (Variables|UFRestricted|GetHome)))
          (Default|Return _asufflag_stand _asufcharacter false)
          (else
            (bind _asufflag_stand_2 (Utilities|Casting|CastToUFFlagStand (Variables|UFRestricted|GetHome)))
            (Default|TakeFlag _asufflag_stand_2 _asufcharacter)))))))

(event Custom|Dropped
  (Variables|UFRestricted|SetbRecentDrop true)
  (Utilities|FlowControl|Delay 1.0)
  (Variables|UFRestricted|SetbRecentDrop false))

(event Custom|StartReset
  (Timeline|DroppedResetDelay PlayFromStart
    (:Finished
      (Variables|/Game/SourceForts/Blueprints/Flags/UFFlagStand.UFFlagStand_C|SetFlagState (Variables|UFRestricted|GetHome) "Base"))))

(event Custom|StopReset
  (Timeline|DroppedResetDelay Stop
    (:Finished
      (Variables|/Game/SourceForts/Blueprints/Flags/UFFlagStand.UFFlagStand_C|SetFlagState (Variables|UFRestricted|GetHome) "Base"))))

(event EventBeginPlay
  (CallFunction|SetColors))

(event EventEndPlay
  (params (EndPlayReason :type EEndPlayReason%20Enum :default "ActorDestroyed"))
  (if (Utilities|Enum|Equal(Enum) EndPlayReason "ActorDestroyed")
    (Default|CreateFlag (Variables|UFRestricted|GetHome))))

(fn ConstructionScript)

(fn OnRepFlagState
  (Utilities|CheckFlagState
    (:Base
      (Class|Actor|DetachRootComponentfromParent true)
      (Physics|SetSimulatePhysics false)
      (Transformation|SetWorldLocation (Transformation|GetWorldLocation (Variables|UFRestricted|GetHome)) false)
      (Transformation|SetWorldScale3D "1.000000,1.000000,1.000000")
      (Networking|SwitchHasAuthority :!label _label
        (:Authority
          (CallFunction|StopReset))))
    (:Taken
      (Physics|SetSimulatePhysics false)
      (Class|Actor|AttachRootComponenttoActor (Variables|UFRestricted|GetCarrier) "None" "SnapToTarget" true)
      (Transformation|SetRelativeTransform (Variables|Default|GetUFFlag) (Math|Transform|MakeTransform "0, 0,250.000000" "0, 0, 0" "1.000000,1.000000,1.000000") false)
      (goto _label))
    (:Dropped
      (Class|Actor|DetachRootComponentfromParent true)
      (Transformation|SetWorldScale3D "1.000000,1.000000,1.000000")
      (Physics|SetSimulatePhysics true)
      (Networking|SwitchHasAuthority
        (:Authority
          (CallFunction|StartReset))))))

(fn SetColors
  (bind _teamnum (Variables|UFRestricted|GetTeamNum))
  (Rendering|Material|SetMaterial (Variables|Default|GetUFFlag) 0 (Utilities|Select :Index _teamnum :Option%200 "/Game/SourceForts/Materials/M_Dev_RedTeam.M_Dev_RedTeam" :Option%201 "/Game/SourceForts/Materials/M_Dev_BlueTeam.M_Dev_BlueTeam"))
  (bind _returnvalue (Rendering|Material|CreateDynamicMaterialInstance 0 0 :!class /Script/Engine.PrimitiveComponent))
  (Rendering|Material|SetScalarParameterValue _returnvalue "Brightness" 5.0 :!class /Script/Engine.MaterialInstanceDynamic)
  (Rendering|Components|Light|SetLightColor (Variables|Default|GetPointLight) (Utilities|Select :Index _teamnum :Option%200 "(R=0.745098,G=0.000000,B=0.000000,A=1.000000)" :Option%201 "(R=0.157000,G=0.356863,B=0.949020,A=1.000000)"))
  (return))