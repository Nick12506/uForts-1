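; BP_AdditiveDummy is a damage test dummy that displays a running total of the damage it takes.
; Each hit adds rounded damage to a string total and restarts the Reset timeline, whose track drives the displayed timer.
; When the timeline finishes, both total and timer return to zero.
; RepNotify functions on both strings update the DamageTaken and Time text displays.
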(event EventAnyDamage
  (params (Damage :type Float%20%28single-precision%29) (DamageType :type Damage%20Type%20Object%20Reference) (InstigatedBy :type Controller%20Object%20Reference) (DamageCauser :type Actor%20Object%20Reference))
  (Variables|Default|SetDamageValue (Utilities|String|ToString(Integer) (Math|Float|Round (+ Damage (Math|Conversions|ToFloat(Integer) (Variables|Default|GetDamageValue))))))
  (bind _newtrack_0 (Timeline|Reset PlayFromStart)
    (:Update
      (Variables|Default|SetTimer (Utilities|String|ToString(Integer) (Math|Float|Ceil _newtrack_0))))
    (:Finished
      (Variables|Default|SetDamageValue "0")
      (Variables|Default|SetTimer "0"))))

(fn ConstructionScript)

(fn OnRepDamageValue
  (Rendering|Components|TextRender|SetText (Variables|Default|GetDamageTaken) (Utilities|String|Append "Damage: " (Variables|Default|GetDamageValue))))

(fn OnRepTimer
  (Rendering|Components|TextRender|SetText (Variables|Default|GetTime) (Utilities|String|Append "Reset: " (Variables|Default|GetTimer))))