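; Big screen mesh Blueprint for the Overload map content, built to bob vertically around its placed position.
; The construction script caches the initial world location.
; A ping-pong Timeline lerps the height slightly above and below that point, reversing each time it finishes.
; Nothing in the graph starts the Timeline, so the bobbing logic never runs.
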(fn ConstructionScript
  (Variables|Default|SetInitialLocation (Transformation|GetWorldLocation)))