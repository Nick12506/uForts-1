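; BP_GrenadeProj is the grenade launcher projectile, a short-lived stand-in that hands off to a physics-driven GrenadeObject.
; On BeginPlay, the server spawns a scaled-down GrenadeObject at the projectile's location and rotation, copying over its velocity and instigator.
; The projectile then destroys itself after a brief delay, leaving the spawned object to carry on.
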(event EventBeginPlay
  (bind _returnvalue (Transformation|GetActorTransform))
  (bind (_location _rotation) (Math|Transform|BreakTransform _returnvalue))
  (Networking|SwitchHasAuthority
    (:Authority
      (bind _returnvalue_2 (Game|SpawnActorfromClass "/Game/SourceForts/Weapons/GrenadeLauncher/GrenadeObject.GrenadeObject_C" (Math|Transform|MakeTransform _location _rotation "0.150000,0.150000,0.150000") false 0))
      (Class|PrimitiveComponent|SetAllPhysicsLinearVelocity _returnvalue_2 (Transformation|GetVelocity) false)
      (Variables|/Script/Engine.Actor|SetInstigator _returnvalue_2 (Variables|Default|GetInstigator))
      (Utilities|FlowControl|Delay 0.2)
      (Actor|DestroyActor))))

(fn ConstructionScript)