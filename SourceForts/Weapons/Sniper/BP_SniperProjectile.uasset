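; Sniper weapon projectile Blueprint that tints its visual effects to the firing character's team.
; On BeginPlay it casts the Instigator to UFCharacter and sets the projectile particle's color from the team number, red or blue.
; On each ProjectileMovement bounce it spawns a bounce emitter at the impact, oriented from the collision component toward the hit point, and applies the same team tint to its color parameters.
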(event OnProjectileBounce(ProjectileMovement)
  (params (ImpactResult :type Hit%20Result%20Structure%20%28by%20ref%29) (ImpactVelocity :type Vector%20%28by%20ref%29 :default "0, 0, 0"))
  (bind _location (Collision|BreakHitResult ImpactResult))
  (bind _returnvalue (Effects|SpawnEmitteratLocation (Variables|Default|GetUFBounceEffect) _location (Math|Rotator|FindLookatRotation (Transformation|GetWorldLocation (Variables|Default|GetCollisionComp)) _location)))
  (bind _asufcharacter (Utilities|Casting|CastToUFCharacter (Variables|Default|GetInstigator)))
  (Effects|Components|ParticleSystem|SetColorParameter _returnvalue "Color1" (Utilities|Select :Index (Class|UTCharacter|GetTeamNum _asufcharacter) :Option%200 "(R=10.000000,G=0.000000,B=0.000000,A=1.000000)" :Option%201 "(R=0.200000,G=0.100000,B=10.000000,A=1.000000)"))
  (Effects|Components|ParticleSystem|SetColorParameter _returnvalue "Color2" (Utilities|Select :Index (Class|UTCharacter|GetTeamNum _asufcharacter) :Option%200 "(R=10.000000,G=0.000000,B=0.000000,A=1.000000)" :Option%201 "(R=0.200000,G=0.100000,B=10.000000,A=1.000000)"))
  (Effects|Components|ParticleSystem|SetColorParameter _returnvalue "Color3" (Utilities|Select :Index (Class|UTCharacter|GetTeamNum _asufcharacter) :Option%200 "(R=10.000000,G=0.000000,B=0.000000,A=1.000000)" :Option%201 "(R=0.200000,G=0.100000,B=10.000000,A=1.000000)"))
  (Effects|Components|ParticleSystem|SetColorParameter _returnvalue "Color4" (Utilities|Select :Index (Class|UTCharacter|GetTeamNum _asufcharacter) :Option%200 "(R=10.000000,G=0.000000,B=0.000000,A=1.000000)" :Option%201 "(R=0.200000,G=0.100000,B=10.000000,A=1.000000)"))
  (Effects|Components|ParticleSystem|SetColorParameter _returnvalue "Color5" (Utilities|Select :Index (Class|UTCharacter|GetTeamNum _asufcharacter) :Option%200 "(R=10.000000,G=0.000000,B=0.000000,A=1.000000)" :Option%201 "(R=0.200000,G=0.100000,B=10.000000,A=1.000000)")))

(event EventBeginPlay
  (bind _asufcharacter (Utilities|Casting|CastToUFCharacter (Variables|Default|GetInstigator)))
  (Effects|Components|ParticleSystem|SetColorParameter (Variables|Default|GetSniperProjectile) "Color" (Utilities|Select :Index (Class|UTCharacter|GetTeamNum _asufcharacter) :Option%200 "(R=100.000000,G=0.000000,B=0.000000,A=1.000000)" :Option%201 "(R=0.200000,G=0.200000,B=100.000000,A=1.000000)")))

(fn ConstructionScript)